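; BP_DynamicChains procedurally builds a physics-constrained chain of boards toward an editable AttachPoint, entirely in its construction script.
; It aims the placeholder board at that point, then creates NumberOfBoards static meshes, deriving each transform from the previous board and the per-board spacing.
; Two physics constraints, offset along the board's right axis, join each mesh to its predecessor.
; The last board has physics simulation disabled, anchoring that end.
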(event EventBeginPlay)

(event Collision|EventActorBeginOverlap
  (params (OtherActor :type Actor%20Object%20Reference)))

(event EventTick
  (params (DeltaSeconds :type Float%20%28single-precision%29)))

(fn ConstructionScript
  (Transformation|SetRelativeRotation (Variables|Default|GetBoardPH) (Math|Rotator|FindLookatRotation (Math|Vector|MakeVector 0.0 0.0 0.0) (Variables|Default|GetAttachPoint)) false false)
  (Variables|Default|SetFinalBoard (Variables|Default|GetBoardPH))
  (for _index (range 1 (Variables|Default|GetNumberOfBoards))
    (bind _returnvalue (CallFunction|CreateStaticMesh (Transformation|GetRelativeTransform (Variables|Default|GetFinalBoard))))
    (CallFunction|CreatePhysicsConstraint (Transformation|GetRelativeTransform (Variables|Default|GetFinalBoard)) _returnvalue (Variables|Default|GetFinalBoard) false)
    (CallFunction|CreatePhysicsConstraint (Transformation|GetRelativeTransform (Variables|Default|GetFinalBoard)) _returnvalue (Variables|Default|GetFinalBoard) false)
    (Variables|Default|SetFinalBoard _returnvalue))
  (Physics|SetSimulatePhysics (Variables|Default|GetFinalBoard) false))

(fn CreateStaticMesh
  (params (InputPin :type Transform))
  (bind _attachpoint (Variables|Default|GetAttachPoint))
  (bind _attachpoint_2 (Variables|Default|GetAttachPoint))
  (bind _numberofboards (Variables|Default|GetNumberOfBoards))
  (bind _returnvalue (Math|Vector|GetUnitDirection(Vector) "0, 0, 0" _attachpoint))
  (bind _returnvalue_2 (Math|Vector|VectorLength _attachpoint_2))
  (bind _returnvalue_3 (/ _returnvalue_2 _numberofboards))
  (bind _returnvalue_4 (* _returnvalue _returnvalue_3))
  (bind _returnvalue_5 (/ (.location InputPin) _returnvalue_4))
  (bind _returnvalue_6 (Math|Transform|MakeTransform _returnvalue_5 (.rotation InputPin) (.scale InputPin)))
  (bind _returnvalue_7 (AddComponent|AddStaticMeshComponent false _returnvalue_6))
  (return _returnvalue_7 _returnvalue_6))

(fn CreatePhysicsConstraint
  (params (BoardPHTransform :type Transform) (Comp1 :type Primitive%20Component%20Object%20Reference) (Comp2 :type Primitive%20Component%20Object%20Reference) (LeftPhysicsConstraint :type Boolean))
  (bind _returnvalue (Math|Vector|GetRightVector (.rotation BoardPHTransform)))
  (bind _returnvalue_2 (AddComponent|AddPhysicsConstraintComponent false (Math|Transform|MakeTransform (+ (* (Math|Vector|SelectVector (* _returnvalue -1.0) _returnvalue LeftPhysicsConstraint) 0.1) (.location BoardPHTransform)) (.rotation BoardPHTransform) "1.000000,1.000000,1.000000")))
  (Class|PhysicsConstraintComponent|SetConstrainedComponents _returnvalue_2 Comp1 "None" Comp2 "None"))